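; Actor component that gives the first-person character a photo viewfinder for taking and holding a single picture.
; On BeginPlay it adds the photo input context, creates the camera widget and attaches a manually triggered SceneCapture2D, targeting RT_Photo1, to the owner's camera.
; Holding zoom shows the viewfinder; capture renders one frame and spawns an attached A_Photo.
; Capturing again destroys that photo, with HasPhoto mirrored to FirstPersonChr.
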(event `self.ReceiveBeginPlay`
  (bind _asscenecapture2d (`self.AsSceneCapture2D`))
  (`EnhancedInputSubsystemInterface.AddMappingContext` (pcsubsystem `EnhancedInputLocalPlayerSubsystem` (`GameplayStatics.GetPlayerController` 0)) "/Game/Inputs/IMC_Photo.IMC_Photo" 0 (struct))
  (bind _returnvalue (`|CreateWidget` "/Game/Camera/UMG_Camera.UMG_Camera_C"))
  (set `self.AsUMGCamera` _returnvalue)
  (bind _returnvalue_2 (`|AddComponentByClass` (`self.GetOwner`) "/Script/Engine.SceneCaptureComponent2D" true (`KismetMathLibrary.MakeTransform` (10.0 0.0 0.0))))
  (set `self.AsSceneCapture2D` _returnvalue_2)
  (`SceneComponent.K2_AttachToComponent` (`self.AsSceneCapture2D`) (`Actor.GetComponentByClass` (`self.GetOwner`) "/Script/Engine.CameraComponent") "None" "KeepRelative" "KeepRelative" "KeepRelative" true)
  (set `SceneCaptureComponent2D.TextureTarget` "/Game/Camera/RT_Photo1.RT_Photo1" _asscenecapture2d)
  (set `SceneCaptureComponent.bCaptureEveryFrame` false _asscenecapture2d)
  (set `SceneCaptureComponent.bCaptureOnMovement` false _asscenecapture2d)
  (set `SceneCaptureComponent.bAlwaysPersistRenderingState` true _asscenecapture2d)
  (set `SceneCaptureComponent2D.FOVAngle` 23.5 _asscenecapture2d))

(event `EnhancedInput|/Game/Inputs/IA_Zoom`
  (params (ActionValue :type Boolean) (ElapsedSeconds :type "Float (double-precision)") (TriggeredSeconds :type "Float (double-precision)") (InputAction :type "InputAction Object Reference" :default "/Game/Inputs/IA_Zoom.IA_Zoom"))
  (:`Started`
    (bind _asfirst_person_chr (cast `/Game/Camera/FirstPersonChr` (`GameplayStatics.GetPlayerPawn` 0)))
    (if (`/Game/Camera/FirstPersonChr.isFirstPerson` _asfirst_person_chr)
      (if (not (`self.HasPhoto`))
        (set `self.isTakingPicture` true)
        (set `self.isZoomedIn` true)
        (bind _asfirst_person_chr_2 (cast `/Game/Camera/FirstPersonChr` (`GameplayStatics.GetPlayerPawn` 0)))
        (if (`/Game/Camera/FirstPersonChr.isFirstPerson` _asfirst_person_chr_2)
          (if (not (`self.HasPhoto`))
            (`UserWidget.AddToViewport` (`self.AsUMGCamera`) 0))))))
  (:`Completed`
    (if (not (`self.HasPhoto`))
      (`Widget.RemoveFromParent` (`self.AsUMGCamera`))
      (set `self.isTakingPicture` false)
      (set `self.isZoomedIn` false))))

(event `EnhancedInput|/Game/Inputs/IA_Capture`
  (params (ActionValue :type Boolean) (ElapsedSeconds :type "Float (double-precision)") (TriggeredSeconds :type "Float (double-precision)") (InputAction :type "InputAction Object Reference" :default "/Game/Inputs/IA_Capture.IA_Capture"))
  (:`Started`
    (bind _asfirst_person_chr (cast `/Game/Camera/FirstPersonChr` (`GameplayStatics.GetPlayerPawn` 0)))
    (if (`/Game/Camera/FirstPersonChr.isFirstPerson` _asfirst_person_chr)
      (if (`self.HasPhoto`)
        (`self.Place Photo`)
        (elif (`Widget.IsVisible` (`self.AsUMGCamera`))
          (set `self.isZoomedIn` false)
          (`self.Capture Photo`)
          (`Widget.RemoveFromParent` (`self.AsUMGCamera`))
          (set `self.isTakingPicture` false))))))

(fn `Capture Photo`
  (bind _returnvalue (`|SpawnActorFromClass` "/Game/Camera/A_Photo.A_Photo_C" (`KismetMathLibrary.MakeTransform` (0.0 0.0 0.0)) "Undefined" "MultiplyWithRoot" null null))
  (bind _output_get (set `self.As A_Photo` _returnvalue))
  (`Actor.K2_AttachToComponent` _output_get (`self.AsSceneCapture2D`) "None" "KeepRelative" "KeepRelative" "KeepRelative" false)
  (`Actor.K2_SetActorRelativeLocation` (`self.As A_Photo`) (45.0 -30.0 -15.0) false true)
  (`SceneCaptureComponent2D.CaptureScene` (`self.AsSceneCapture2D`))
  (bind _output_get_2 (set `self.HasPhoto` true))
  (bind _asfirst_person_chr (cast `/Game/Camera/FirstPersonChr` (`GameplayStatics.GetPlayerPawn` 0)))
  (set `/Game/Camera/FirstPersonChr.hasPhoto` _output_get_2 _asfirst_person_chr))

(fn `Place Photo`
  (bind _output_get (set `self.HasPhoto` false))
  (bind _asfirst_person_chr (cast `/Game/Camera/FirstPersonChr` (`GameplayStatics.GetPlayerPawn` 0)))
  (set `/Game/Camera/FirstPersonChr.hasPhoto` _output_get _asfirst_person_chr)
  (`Actor.K2_DestroyActor` (`self.As A_Photo`)))